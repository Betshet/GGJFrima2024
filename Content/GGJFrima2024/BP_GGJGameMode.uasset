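; BP_GGJGameMode is a game mode Blueprint for the GGJFrima2024 game that tracks intro completion and sets up dialogue for the player and an NPC.
; On BeginPlay it finds and stores the BP_Character as the player and the BP_NPC as Max.
; FinishIntro runs its logic only once, assigning the D_Dialogues graph to both Mountea dialogue participants and then flagging the intro as finished.
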(event Custom|FinishIntro
  (if (not (Variables|Default|GetbHasFinishedIntro))
    (Class|MounteaDialogueParticipant|SetDialogueGraph (Variables|/Game/DialogueSystem/Bluprints/BP_Character.BP_Character_C|GetMounteaDialogueParticipant (Variables|Default|GetPlayerCharacter)) "/Game/DialogueSystem/Dialogues/D_Dialogues.D_Dialogues")
    (Class|MounteaDialogueParticipant|SetDialogueGraph (Variables|/Game/DialogueSystem/Bluprints/BP_NPC.BP_NPC_C|GetMounteaDialogueParticipant (Variables|Default|GetMax)) "/Game/DialogueSystem/Dialogues/D_Dialogues.D_Dialogues")
    (Variables|Default|SetbHasFinishedIntro true)))

(event EventBeginPlay
  (bind _returnvalue (Actor|GetActorOfClass "/Game/DialogueSystem/Bluprints/BP_Character.BP_Character_C"))
  (Variables|Default|SetPlayerCharacter _returnvalue)
  (bind _returnvalue_2 (Actor|GetActorOfClass "/Game/DialogueSystem/Bluprints/BP_NPC.BP_NPC_C"))
  (Variables|Default|SetMax _returnvalue_2))

(fn ConstructionScript)