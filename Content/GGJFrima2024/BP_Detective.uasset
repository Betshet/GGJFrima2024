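; First-person detective player Blueprint that handles object interaction, item inspection, inventory and a "detective vision" ability.
; A camera line trace finds InteractiveComponent actors, either entering rotatable viewing or adding them to the player controller's inventory and destroying them.
; Viewing and inventory modes push and remove prioritized Enhanced Input mapping contexts.
; Vision temporarily spawns copies of "Souvenir"-tagged meshes with a special material, destroying them after five seconds.
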(event Custom|LetGo
  (bind _asplayer_controller (Utilities|Casting|CastToPlayerController (Pawn|GetController)))
  (Utilities|IsValid (PlayerController|LocalPlayerSubsystems|GetEnhancedInputLocalPlayerSubsystem _asplayer_controller)
    (:Is%20Valid
      (Input|RemoveMappingContext (PlayerController|LocalPlayerSubsystems|GetEnhancedInputLocalPlayerSubsystem _asplayer_controller) "/Game/PIerre_InventorySystem/IMC_ViewingItem.IMC_ViewingItem" "(bIgnoreAllPressedKeysUntilRelease=True,bForceImmediately=False,bNotifyUserSettings=False)")
      (bind _asstatic_mesh_component (Utilities|Casting|CastToStaticMeshComponent (Variables|Default|GetGrabbedComponent)))
      (Collision|SetCollisionEnabled _asstatic_mesh_component "QueryAndPhysics")
      (Physics|SetSimulatePhysics _asstatic_mesh_component true)
      (Default|ReturntoPOsition (Variables|Default|GetInteractiveComponent))
      (Variables|Default|SetGrabbedComponent 0)
      (Variables|Default|SetInteractiveComponent 0)
      (Variables|Holding|SetGrabbedActor 0))))

(event Custom|ViewItem
  (bind _asplayer_controller (Utilities|Casting|CastToPlayerController (Pawn|GetController)))
  (Utilities|IsValid (PlayerController|LocalPlayerSubsystems|GetEnhancedInputLocalPlayerSubsystem _asplayer_controller)
    (:Is%20Valid
      (Input|AddMappingContext (PlayerController|LocalPlayerSubsystems|GetEnhancedInputLocalPlayerSubsystem _asplayer_controller) "/Game/PIerre_InventorySystem/IMC_ViewingItem.IMC_ViewingItem" 10 "(bIgnoreAllPressedKeysUntilRelease=True,bForceImmediately=False,bNotifyUserSettings=False)"))))

(event Input|EnhancedActionEvents|EnhancedInputActionIA_Vision
  (params (ActionValue :type Boolean) (ElapsedSeconds :type Float%20%28double-precision%29) (TriggeredSeconds :type Float%20%28double-precision%29) (InputAction :type Input%20Action%20Object%20Reference :default "/Game/FirstPerson/Input/Actions/IA_Vision.IA_Vision"))
  (bind _spawnedactors_0 (Variables|Default|GetSpawnedActors_0))
  ;[1 1 1] Detective vision
  (:Started
    (bind _outactors (Actor|GetAllActorsOfClasswithTag "/Script/Engine.StaticMeshActor" "Souvenir"))
    (for _array_element _outactors
      (bind _returnvalue (Game|SpawnActorfromClass (Utilities|GetClass _array_element) (Transformation|GetActorTransform _array_element) "AlwaysSpawn" "MultiplyWithRoot" 0 0))
      (Utilities|Array|Add (Variables|Default|GetSpawnedActors_0) _returnvalue)
      (Transformation|SetMobility _returnvalue "Movable")
      (Components|StaticMesh|SetStaticMesh (Variables|/Script/Engine.StaticMeshActor|GetStaticMeshComponent _returnvalue) (Variables|/Script/Engine.StaticMeshComponent|GetStaticMesh (Variables|/Script/Engine.StaticMeshActor|GetStaticMeshComponent _array_element)))
      (Rendering|Material|SetMaterial (Variables|/Script/Engine.StaticMeshActor|GetStaticMeshComponent _returnvalue) 0 "/Game/LevelPrototyping/Materials/M_Souvenir.M_Souvenir"))
    (Utilities|FlowControl|Delay 5.0)
    (for _array_element_2 _spawnedactors_0
      (Actor|DestroyActor _array_element_2))
    (Utilities|Array|Clear _spawnedactors_0)))

(event Input|EnhancedActionEvents|EnhancedInputActionIA_Viewing
  (params (ActionValue :type Vector%202D%20Structure) (ElapsedSeconds :type Float%20%28double-precision%29) (TriggeredSeconds :type Float%20%28double-precision%29) (InputAction :type Input%20Action%20Object%20Reference :default "/Game/FirstPerson/Input/Actions/IA_Viewing.IA_Viewing"))
  (bind (_x _y) (Math|Vector2D|BreakVector2D ActionValue))
  (bind _asstatic_mesh_component (Utilities|Casting|CastToStaticMeshComponent (Variables|Default|GetGrabbedComponent)))
  (Physics|SetSimulatePhysics _asstatic_mesh_component false)
  (Collision|SetCollisionEnabled _asstatic_mesh_component "NoCollision")
  (Transformation|AddWorldRotation _asstatic_mesh_component (Math|Rotator|MakeRotator _y 0.0 _x) false true))

(event Input|EnhancedActionEvents|EnhancedInputActionIA_Test
  (params (ActionValue :type Boolean) (ElapsedSeconds :type Float%20%28double-precision%29) (TriggeredSeconds :type Float%20%28double-precision%29) (InputAction :type Input%20Action%20Object%20Reference :default "/Game/FirstPerson/Input/Actions/IA_Test.IA_Test"))
  (Development|PrintString "test action")
  (CallFunction|LetGo))

(event Input|EnhancedActionEvents|EnhancedInputActionIA_ToggleInventory
  (params (ActionValue :type Boolean) (ElapsedSeconds :type Float%20%28double-precision%29) (TriggeredSeconds :type Float%20%28double-precision%29) (InputAction :type Input%20Action%20Object%20Reference :default "/Game/PIerre_InventorySystem/IA_ToggleInventory.IA_ToggleInventory"))
  (:Started
    (bind _output_get (Variables|Default|SetIsInventoryOpen (not (Variables|Default|GetIsInventoryOpen))))
    (CallFunction|ToggleInventory _output_get)))

(event Input|EnhancedActionEvents|EnhancedInputActionIA_Interact
  (params (ActionValue :type Boolean) (ElapsedSeconds :type Float%20%28double-precision%29) (TriggeredSeconds :type Float%20%28double-precision%29) (InputAction :type Input%20Action%20Object%20Reference :default "/Game/FirstPerson/Input/Actions/IA_Interact.IA_Interact"))
  (bind _firstpersoncameracomponent (Variables|Default|GetFirstPersonCameraComponent))
  (bind _returnvalue (Math|Vector|GetForwardVector _firstpersoncameracomponent))
  (bind _returnvalue_2 (Transformation|GetWorldLocation _firstpersoncameracomponent))
  (bind _returnvalue_3 (* _returnvalue 5e+02))
  (bind _returnvalue_4 (+ _returnvalue_2 _returnvalue_3))
  (Development|PrintString "trying to interact")
  (Rendering|Debug|DrawDebugLine _returnvalue_2 _returnvalue_4 "(R=1.000000,G=0.000000,B=0.883861,A=1.000000)" 1.0 1e+01)
  (bind _outhit (Collision|LineTraceByChannel _returnvalue_2 _returnvalue_4 "TraceTypeQuery1" false 0 "None"))
  (if (.bBlockingHit (Collision|BreakHitResult _outhit))
    (Utilities|IsValid (Actor|GetComponentbyClass (.HitActor (Collision|BreakHitResult _outhit)) "/Game/PIerre_InventorySystem/InteractiveComponent.InteractiveComponent_C")
      (:Is%20Valid
        ;[1 1 1] Incase we want to object to do something
        (Default|ActivateInteractable (Actor|GetComponentbyClass (.HitActor (Collision|BreakHitResult _outhit)) "/Game/PIerre_InventorySystem/InteractiveComponent.InteractiveComponent_C"))
        (switch Utilities|FlowControl|Switch|SwitchonBPEnum_InteractionType (Variables|/Game/PIerre_InventorySystem/InteractiveComponent.InteractiveComponent_C|GetInteractionType (Actor|GetComponentbyClass (.HitActor (Collision|BreakHitResult _outhit)) "/Game/PIerre_InventorySystem/InteractiveComponent.InteractiveComponent_C"))
          (:NewEnumerator1
            (Development|PrintString "view item")
            (bind _output_get (Variables|Holding|SetGrabbedActor (.HitActor (Collision|BreakHitResult _outhit))))
            (Variables|Default|SetInteractiveComponent (Actor|GetComponentbyClass (.HitActor (Collision|BreakHitResult _outhit)) "/Game/PIerre_InventorySystem/InteractiveComponent.InteractiveComponent_C"))
            (Variables|Default|SetGrabbedComponent (.HitComponent (Collision|BreakHitResult _outhit)))
            (Variables|Default|SetHealdObjectOriginalTransfom (Transformation|GetActorTransform _output_get))
            (CallFunction|ViewItem))
          (:NewEnumerator0
            (Development|PrintString "Add to inventory")
            (bind _output_get_2 (Variables|Holding|SetPIckableItem (.HitActor (Collision|BreakHitResult _outhit))))
            (bind _itemdata (Default|AddItemtoInventory (Variables|Default|GetAs%20BP%20GGJPC) _output_get_2))
            (Actor|DestroyActor _output_get_2)
            (Variables|Default|SetCurrentlySelectedItem _itemdata)))))))

(event Input|EnhancedActionEvents|EnhancedInputActionIA_NavigateInventory
  (params (ActionValue :type Float%20%28double-precision%29) (ElapsedSeconds :type Float%20%28double-precision%29) (TriggeredSeconds :type Float%20%28double-precision%29) (InputAction :type Input%20Action%20Object%20Reference :default "/Game/PIerre_InventorySystem/IA_NavigateInventory.IA_NavigateInventory"))
  (:Started
    (if (Variables|Default|GetIsInventoryOpen)
      (Default|ChangeSelectedItem (Variables|Default|GetAs%20BP%20GGJPC) (> ActionValue 0.0)))))

(event EventBeginPlay
  (bind _asbp_detective_player_controller (Utilities|Casting|CastToBP_DetectivePlayerController (Pawn|GetController)))
  (bind _output_get (Variables|Default|SetAs%20BP%20GGJPC _asbp_detective_player_controller))
  (Utilities|IsValid (PlayerController|LocalPlayerSubsystems|GetEnhancedInputLocalPlayerSubsystem _output_get)
    (:Is%20Valid
      (Input|AddMappingContext (PlayerController|LocalPlayerSubsystems|GetEnhancedInputLocalPlayerSubsystem _output_get) "/Game/PIerre_InventorySystem/IMC_Interaction.IMC_Interaction" 0 "(bIgnoreAllPressedKeysUntilRelease=True,bForceImmediately=False,bNotifyUserSettings=False)"))))

(fn ConstructionScript)

(fn ToggleInventory
  (params (Condition :type Boolean))
  (bind _as_bp_ggjpc (Variables|Default|GetAs%20BP%20GGJPC))
  (bind _viewinventorymapping (Variables|Default|GetViewInventoryMapping))
  (bind _returnvalue (PlayerController|LocalPlayerSubsystems|GetEnhancedInputLocalPlayerSubsystem _as_bp_ggjpc))
  (bind _output_get (Variables|Default|SetIsInventoryOpen Condition))
  (if _output_get
    (Default|ToggleInventoryPlayerController _as_bp_ggjpc true)
    (Utilities|IsValid _returnvalue
      (:Is%20Valid
        (Input|AddMappingContext _returnvalue _viewinventorymapping 3 "(bIgnoreAllPressedKeysUntilRelease=True,bForceImmediately=False,bNotifyUserSettings=False)")))
    (else
      (Default|ToggleInventoryPlayerController _as_bp_ggjpc false)
      (Utilities|IsValid _returnvalue
        (:Is%20Valid
          (Input|RemoveMappingContext _returnvalue _viewinventorymapping "(bIgnoreAllPressedKeysUntilRelease=True,bForceImmediately=False,bNotifyUserSettings=False)"))))))