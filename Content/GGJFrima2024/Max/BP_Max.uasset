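; BP_Max is an interactive NPC character that wanders, sits and talks.
; It walks to a random Waypoint, then to the SittingWaypoint, and stands after a retriggerable delay unless talking.
; Interaction halts movement and starts a Mountea dialogue; StopDialogue resumes sitting or walking.
; Tick writes its position to MPC_NPCUtils, world location overwriting screen position, and player-controller input and inventory logic is also present.
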(event Custom|OnComponentInteracted
  (CallFunction|StartDialogue))

(event Custom|StandUp
  ;[1 1 1] AI Navigation
  (Variables|Navigation|SetbShouldSitDown false))

(event Custom|SitDown
  ;[1 1 1] AI Navigation
  (Variables|Navigation|SetbShouldSitDown true)
  (Utilities|FlowControl|RetriggerableDelay 1e+01 :!label _label)
  (if (Variables|Navigation|GetbIsTalking)
    (goto _label)
    (else
      (CallFunction|StandUp))))

(event Custom|SetupNavigation
  ;[1 1 1] AI Navigation
  (bind _outactors (Actor|GetAllActorsOfClass "/Game/GGJFrima2024/Max/Waypoint.Waypoint_C"))
  (Variables|Navigation|SetWaypoints _outactors)
  (bind _returnvalue (Actor|GetActorOfClass "/Game/GGJFrima2024/Max/SittingWaypoint.SittingWaypoint_C"))
  (Variables|Navigation|SetSittingWaypoint _returnvalue)
  (CallFunction|WalkAround))

(event Custom|StartDialogue
  (Variables|Navigation|SetbIsTalking true)
  (Components|Movement|StopMovementImmediately (Variables|Character|GetCharacterMovement))
  (bind _returnvalue (Class|MounteaDialogueSystemBFC|InitializeDialogue self (Variables|Default|GetMounteaDialogueParticipant)))
  (if _returnvalue
    (Development|PrintString "True")
    (else
      (Development|PrintString "False"))))

(event Custom|WalkAround
  (bind _self self)
  (bind _sittingwaypoint (Variables|Navigation|GetSittingWaypoint))
  ;[1 1 1] AI Navigation
  (AI|AIMoveTo self "0, 0, 0" (.OutItem (Utilities|Array|Random (Variables|Navigation|GetWaypoints))) 5.0 false
    (:OnSuccess
      (Utilities|FlowControl|Delay 5.0)
      (AI|AIMoveTo _self "0, 0, 0" _sittingwaypoint 5.0 false
        (:OnSuccess
          (Transformation|SetActorRotation _self (Transformation|GetActorRotation _sittingwaypoint))
          (CallFunction|SitDown))))))

(event Custom|StopDialogue
  ;[1 1 1] AI Navigation
  (Variables|Navigation|SetbIsTalking false)
  (if (Variables|Navigation|GetbShouldSitDown)
    (CallFunction|SitDown)
    (else
      (CallFunction|WalkAround))))

(event Custom|ResumeSitDown
  ;[1 1 1] AI Navigation
  (Utilities|FlowControl|RetriggerableDelay 1e+01 :!label _label)
  (if (Variables|Navigation|GetbIsTalking)
    (goto _label)
    (else
      (CallFunction|StandUp))))

(event EventBeginPlay
  (CallFunction|SetupNavigation)
  (EventDispatchers|BindEventtoComponentInteracted (Variables|Default|GetInteractiveComponent) (delegate Custom|OnComponentInteracted))
  (bind _asbp_detective_player_controller (Utilities|Casting|CastToBP_DetectivePlayerController (Pawn|GetController)))
  (bind _output_get (Variables|Default|SetAs%20BP%20First%20Person%20Player%20Controller%20Pierr%20Test _asbp_detective_player_controller))
  (Utilities|IsValid (PlayerController|LocalPlayerSubsystems|GetEnhancedInputLocalPlayerSubsystem _output_get)
    (:Is%20Valid
      (Input|AddMappingContext (PlayerController|LocalPlayerSubsystems|GetEnhancedInputLocalPlayerSubsystem _output_get) "/Game/PIerre_InventorySystem/IMC_Interaction.IMC_Interaction" 0 "(bIgnoreAllPressedKeysUntilRelease=True,bForceImmediately=False,bNotifyUserSettings=False)"))))

(event EventTick
  (params (DeltaSeconds :type Float%20%28single-precision%29))
  (bind _returnvalue (Transformation|GetActorLocation))
  (Rendering|Material|SetVectorParameterValue "/Game/LevelPrototyping/Materials/MPC_NPCUtils.MPC_NPCUtils" "NPCPosition" (Math|Conversions|ToLinearColor(Vector) (Math|Conversions|ToVector(Vector2D) (/ (.ScreenLocation (Class|PlayerController|ProjectWorldLocationtoScreen (Game|GetPlayerController 0) _returnvalue false)) "(X=1100.000000,Y=700.000000)"))) :!class /Script/Engine.KismetMaterialLibrary)
  (Rendering|Material|SetVectorParameterValue "/Game/LevelPrototyping/Materials/MPC_NPCUtils.MPC_NPCUtils" "NPCPosition" (Math|Conversions|ToLinearColor(Vector) _returnvalue) :!class /Script/Engine.KismetMaterialLibrary))

(fn ConstructionScript)

(fn ToggleInventory
  (params (Condition :type Boolean))
  (bind _as_bp_first_person_player_controller_pierr_test (Variables|Default|GetAs%20BP%20First%20Person%20Player%20Controller%20Pierr%20Test))
  (bind _viewinventorymapping (Variables|Default|GetViewInventoryMapping))
  (bind _returnvalue (PlayerController|LocalPlayerSubsystems|GetEnhancedInputLocalPlayerSubsystem _as_bp_first_person_player_controller_pierr_test))
  (bind _output_get (Variables|Default|SetIsInventoryOpen Condition))
  (if _output_get
    (Default|ToggleInventoryPlayerController _as_bp_first_person_player_controller_pierr_test true)
    (Utilities|IsValid _returnvalue
      (:Is%20Valid
        (Input|AddMappingContext _returnvalue _viewinventorymapping 3 "(bIgnoreAllPressedKeysUntilRelease=True,bForceImmediately=False,bNotifyUserSettings=False)")))
    (else
      (Default|ToggleInventoryPlayerController _as_bp_first_person_player_controller_pierr_test false)
      (Utilities|IsValid _returnvalue
        (:Is%20Valid
          (Input|RemoveMappingContext _returnvalue _viewinventorymapping "(bIgnoreAllPressedKeysUntilRelease=True,bForceImmediately=False,bNotifyUserSettings=False)"))))))