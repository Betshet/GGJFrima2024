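; BP_GGJPC, apparently the game's player controller, keeps the held-item inventory.
; AddItemToInventory reads the item name from an actor's InteractiveComponent, logs it, and adds a unique HeldItem struct storing name, actor class and in-inventory flag.
; HasItem checks name and inventory flag but returns inside its loop, so only the first entry is evaluated.
; BeginPlay and Tick are unused stubs.
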(event EventBeginPlay
  (|CallParentFunction) ; This node is disabled and will not be called.\nDrag off pins to build functionality.
)

(event EventTick
  (params (DeltaSeconds :type Float%20%28single-precision%29)))

(fn ConstructionScript
  (|CallParentFunction))

(fn HasItem
  (params (ItemName :type String))
  (for _array_element (Variables|Default|GetHeldItems)
    (return (and (Utilities|Enum|Equal(Enum) (.ItemName (Utilities|Struct|BreakHeldItem _array_element)) ItemName) (.IsInInventory (Utilities|Struct|BreakHeldItem _array_element))))))

(fn AddItemtoInventory
  (params (Actor :type Actor%20Object%20Reference))
  (bind _returnvalue (Actor|GetComponentbyClass Actor "/Game/PIerre_InventorySystem/InteractiveComponent.InteractiveComponent_C"))
  (bind _itemname (Variables|/Game/PIerre_InventorySystem/InteractiveComponent.InteractiveComponent_C|GetItemName _returnvalue))
  (Development|PrintString (Utilities|String|Append "Adding item to inventory:  " _itemname))
  (Utilities|Array|AddUnique (Variables|Default|GetHeldItems) (Utilities|Struct|MakeHeldItem _itemname (Utilities|GetClass Actor) true false)))