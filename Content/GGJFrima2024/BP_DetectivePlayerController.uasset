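; Player controller for the detective game that owns the player's inventory and links dialogue events to story progress.
; It creates the inventory HUD, seeds a test item, and handles adding, checking, toggling and cycling held items.
; Trigger decorators on finished dialogue nodes complete named history steps in the game mode.
; Closing dialogue finishes the intro if that step is still incomplete.
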(event Custom|ToggleInventory_PlayerController
  (params (IsOPen :type Boolean))
  (bind _hudinventory (Variables|Default|GetHUDInventory))
  (if (and (== (Variables|Default|GetSelectedItemIndex) -1) (> (Class|ListView|GetNumItems (Variables|/Game/PIerre_InventorySystem/HUD/HUD_Inventory.HUD_Inventory_C|GetListView_258 (Variables|Default|GetHUDInventory))) 0))
    (Default|SelectItem _hudinventory)
    (else
      (bind _index (CallFunction|GetSelectedIndex))
      (Variables|Default|SetSelectedItemIndex _index)))
  (Default|HUDToggleInventory _hudinventory IsOPen))

(event Custom|SetupInventory
  (Development|PrintString "Hello")
  (Utilities|Array|AddUnique (Variables|Default|GetHeldItems) (Utilities|Struct|MakeHeldItem "Test Item" true false "" 0 0 0 0))
  (bind _returnvalue (UserInterface|CreateWidget "/Game/PIerre_InventorySystem/HUD/HUD_Inventory.HUD_Inventory_C"))
  (bind _output_get (Variables|Default|SetHUDInventory _returnvalue))
  (UserInterface|Viewport|AddtoViewport _output_get 0))

(event Custom|OnDialogueClosed
  (params (Context :type Mountea%20Dialogue%20Context%20Object%20Reference))
  (Utilities|IsValid Context
    (:Is%20Valid
      (Development|PrintString "Intro Finished")
      (bind _mygamemode (CallFunction|GetMyGamemode))
      (bind _bisdone (Default|IsHistoryStepComplete _mygamemode "Intro"))
      (if (not _bisdone)
        (Default|FinishIntro _mygamemode)))))

(event Custom|OnNodeFinished
  (params (Context :type Mountea%20Dialogue%20Context%20Object%20Reference))
  (bind _activenode (Variables|/Script/MounteaDialogueSystem.MounteaDialogueContext|GetActiveNode Context))
  (Utilities|IsValid Context
    (:Is%20Valid
      (Utilities|IsValid _activenode
        (:Is%20Valid
          (bind _array_element (Utilities|Array|ForEachLoopwithBreak (Variables|/Script/MounteaDialogueSystem.MounteaDialogueGraphNode|GetNodeDecorators _activenode))
            (:LoopBody
              (bind _astrigger_on_finish (Utilities|Casting|CastToDecorator_Trigger (Utilities|Struct|BreakMounteaDialogueDecorator _array_element)))
              (bind _mygamemode (CallFunction|GetMyGamemode))
              (Default|CompleteHistoryStep _mygamemode (Variables|/Script/GGJFrima2024.Decorator_Trigger|GetTriggerName _astrigger_on_finish)))))))))

(event EventBeginPlay
  (|CallParentFunction)
  (CallFunction|SetupInventory)
  (EventDispatchers|BindEventtoOnDialogueClosed (Variables|Default|GetBP_DialogueManager) (delegate Custom|OnDialogueClosed))
  (EventDispatchers|BindEventtoOnDialogueNodeFinished (Variables|Default|GetBP_DialogueManager) (delegate Custom|OnNodeFinished)))

(fn ConstructionScript
  (|CallParentFunction))

(fn HasItem
  (params (ItemName :type String))
  (for _array_element (Variables|Default|GetHeldItems)
    (if (and (Utilities|Enum|Equal(Enum) (.ItemName (Utilities|Struct|BreakHeldItem _array_element)) ItemName) (.IsInInventory (Utilities|Struct|BreakHeldItem _array_element)))
      (return true)))
  (return false))

(fn AddItemtoInventory
  (params (Actor :type Actor%20Object%20Reference))
  (bind _returnvalue (Actor|GetComponentbyClass Actor "/Game/PIerre_InventorySystem/InteractiveComponent.InteractiveComponent_C"))
  (bind _helditemdata (Variables|/Game/PIerre_InventorySystem/InteractiveComponent.InteractiveComponent_C|GetHeldItemData _returnvalue))
  (Default|GetStaticMesh _returnvalue)
  (Development|PrintString (Utilities|String|Append "Adding item to inventory:  " (Variables|/Game/PIerre_InventorySystem/InteractiveComponent.InteractiveComponent_C|GetItemName _returnvalue)))
  (Utilities|Array|AddUnique (Variables|Default|GetHeldItems) _helditemdata)
  (Default|AddItemtoList (Variables|Default|GetHUDInventory) _helditemdata)
  (return _helditemdata))

(fn GetSelectedIndex
  (for (_array_element _array_index) (Class|ListView|GetListItems (Variables|/Game/PIerre_InventorySystem/HUD/HUD_Inventory.HUD_Inventory_C|GetListView_258 (Variables|Default|GetHUDInventory)))
    (bind _asbpw_inventory_item_list (Utilities|Casting|CastToBPW_InventoryItemList _array_element))
    (if (Utilities|AreEqual (Variables|/Game/PIerre_InventorySystem/HUD/BPW_InventoryItemList.BPW_InventoryItemList_C|GetItemData _asbpw_inventory_item_list) (Variables|Default|GetCurrentlySelectedItem))
      (return _array_index)))
  (return -1))

(fn ChangeSelectedItem
  (params (Increase :type Boolean))
  (bind _hudinventory (Variables|Default|GetHUDInventory))
  (if Increase
    (Default|SelectNextItem _hudinventory)
    (else
      (Default|SelectPreviousItem _hudinventory))))