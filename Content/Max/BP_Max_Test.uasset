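; Test AI pawn for Max that walks to a random waypoint, pauses, then goes to a sitting waypoint to sit.
; BeginPlay caches the waypoints and starts the AIMoveTo chain, which ends by matching the seat's rotation and setting ShouldSitDown.
; UpdateMovement clears that flag after a delay; the next trip needs an outside call to OnSittingToIdleComplete.
; Failed moves are unhandled, so they stall the routine.
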(event Custom|UpdateMovement
  (params (bSitDown :type Boolean))
  (if bSitDown
    (Variables|Default|SetbShouldSitDown true)
    (Utilities|FlowControl|Delay 1e+01)
    (CallFunction|UpdateMovement false)
    (else
      (Variables|Default|SetbShouldSitDown false))))

(event Custom|OnSittingToIdleComplete
  (bind _self self)
  (bind _sittingwaypoint (Variables|Default|GetSittingWaypoint))
  (AI|AIMoveTo self "0, 0, 0" (.OutItem (Utilities|Array|Random (Variables|Default|GetWaypoints))) 5.0 false
    (:OnSuccess
      (Utilities|FlowControl|Delay 5.0)
      (AI|AIMoveTo _self "0, 0, 0" _sittingwaypoint 5.0 false
        (:OnSuccess
          (Transformation|SetActorRotation _self (Transformation|GetActorRotation _sittingwaypoint))
          (CallFunction|UpdateMovement true))))))

(event EventBeginPlay
  (bind _outactors (Actor|GetAllActorsOfClass "/Game/Max/Waypoint.Waypoint_C"))
  (Variables|Default|SetWaypoints _outactors)
  (bind _returnvalue (Actor|GetActorOfClass "/Game/Max/SittingWaypoint.SittingWaypoint_C"))
  (Variables|Default|SetSittingWaypoint _returnvalue)
  (CallFunction|OnSittingtoIdleComplete))

(event Collision|EventActorBeginOverlap
  (params (OtherActor :type Actor%20Object%20Reference)))

(event EventTick
  (params (DeltaSeconds :type Float%20%28single-precision%29)))

(fn ConstructionScript)