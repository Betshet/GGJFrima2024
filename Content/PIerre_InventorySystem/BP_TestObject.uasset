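; BP_TestObject is a test actor in the inventory system that responds to interaction through an InteractiveComponent.
; On BeginPlay it binds ObjectInteracted to the component's interacted event.
; The handler switches on InteractionType, but no branch has any behavior wired.
; Disconnected nodes that would turn off the Cube's physics, overlap events and collision remain in the graph and never run.
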(event Custom|ObjectInteracted
  (switch Utilities|FlowControl|Switch|SwitchonBPEnum_InteractionType (Variables|/Game/PIerre_InventorySystem/InteractiveComponent.InteractiveComponent_C|GetInteractionType (Variables|Default|GetInteractiveComponent))))

(event EventBeginPlay
  (EventDispatchers|BindEventtoComponentInteracted (Variables|Default|GetInteractiveComponent) (delegate Custom|ObjectInteracted)))

(fn ConstructionScript)