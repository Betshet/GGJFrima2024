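; Player controller that drives dialogue input, starting a conversation with the BP_Max NPC cached at BeginPlay and advancing lines through the dialogue manager.
; The Speak action starts dialogue, while the Jump action requests the next line.
; Skip key events implement hold-to-skip during active dialogue: pressing shows the skip UI and starts a timer, and releasing cancels both.
; Finishing the hold requests a voice skip and hides the prompt.
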(event Custom|SkipKeyPressed_Event
  (bind _bp_dialoguemanager (Variables|Default|GetBP_DialogueManager))
  ;[1 1 1] Manager User Widget
  (Utilities|IsValid (Class|MounteaDialogueManager|GetDialogueUIPtr (Variables|Default|GetBP_DialogueManager))
    (:Is%20Valid
      (switch Utilities|FlowControl|Switch|SwitchonEDialogueManagerState (Class|MounteaDialogueManager|GetDialogueManagerState (Variables|Default|GetBP_DialogueManager))
        (:EDMS_Active
          (Utilities|Time|ClearandInvalidateTimerbyHandle (Variables|Default|GetTimerHandle_SkipPressed))
          (Class|MounteaDialogueWBPInterface|RefreshDialogueWidget(Message) (Class|MounteaDialogueManager|GetDialogueUIPtr _bp_dialoguemanager) _bp_dialoguemanager "ShowSkipUI")
          (bind _returnvalue (Utilities|Time|SetTimerbyEvent (EventDispatchers|CreateEvent :!event DialogueSkipHoldFinished) (Variables|Default|GetSkipHoldDuration)))
          (Variables|Default|SetTimerHandle_SkipPressed _returnvalue))))))

(event Custom|SkipKeyReleased_Event
  (bind _bp_dialoguemanager (Variables|Default|GetBP_DialogueManager))
  ;[1 1 1] Manager User Widget
  (Utilities|IsValid (Class|MounteaDialogueManager|GetDialogueUIPtr (Variables|Default|GetBP_DialogueManager))
    (:Is%20Valid
      (switch Utilities|FlowControl|Switch|SwitchonEDialogueManagerState (Class|MounteaDialogueManager|GetDialogueManagerState (Variables|Default|GetBP_DialogueManager))
        (:EDMS_Active
          (Utilities|Time|ClearandInvalidateTimerbyHandle (Variables|Default|GetTimerHandle_SkipPressed))
          (Class|MounteaDialogueWBPInterface|RefreshDialogueWidget(Message) (Class|MounteaDialogueManager|GetDialogueUIPtr _bp_dialoguemanager) _bp_dialoguemanager "HideSkipUI"))))))

(event Input|EnhancedActionEvents|EnhancedInputActionIA_Speak
  (params (ActionValue :type Boolean) (ElapsedSeconds :type Float%20%28double-precision%29) (TriggeredSeconds :type Float%20%28double-precision%29) (InputAction :type Input%20Action%20Object%20Reference :default "/Game/FirstPerson/Input/Actions/IA_Speak.IA_Speak"))
  (Default|StartDialogue (Variables|Default|GetNPC)))

(event Input|EnhancedActionEvents|EnhancedInputActionIA_Jump
  (params (ActionValue :type Boolean) (ElapsedSeconds :type Float%20%28double-precision%29) (TriggeredSeconds :type Float%20%28double-precision%29) (InputAction :type Input%20Action%20Object%20Reference :default "/Game/FirstPerson/Input/Actions/IA_Jump.IA_Jump"))
  (:Started
    (Class|MyDialogueManager|NextDialogue (Variables|Default|GetBP_DialogueManager))))

(event EventBeginPlay
  (bind _returnvalue (Actor|GetActorOfClass "/Game/GGJFrima2024/Max/BP_Max.BP_Max_C"))
  (Variables|Default|SetNPC _returnvalue))

(fn ConstructionScript)

(fn DialogueSkipHoldFinished
  (Default|CallOnDialogueVoiceSkipRequest (Variables|Default|GetBP_DialogueManager))
  (Class|MounteaDialogueWBPInterface|RefreshDialogueWidget(Message) (Class|MounteaDialogueManager|GetDialogueUIPtr (Variables|Default|GetBP_DialogueManager)) (Variables|Default|GetBP_DialogueManager) "HideSkipUI"))